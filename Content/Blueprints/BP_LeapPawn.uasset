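; Pawn that drives an animated body's hands from Leap Motion tracking.
; Hand-moved events copy Leap data into AnimBody's left and right sides, converting each with pre and post basis rotations.
; Hand count changes enable each tracked side and hide untracked forearm bones on the skeletal mesh, checking frame hand types when only one is visible.
; Debug keys query, pause and resume tracking.
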(event `self.ReceiveBeginPlay`
  (`AnimBody.SetEnabled` (`self.AnimBody`) true))

(event `LeapEventInterface.LeapLeftHandMoved`
  (params (Hand :type "LeapHand Object Reference"))
  (bind _left (`AnimBody.Left` (`self.AnimBody`)))
  (`AnimHand.SetFromLeapHand` _left Hand)
  (`AnimHand.ChangeBasis` _left (`self.LeftPreBase`) (`self.LeftPostBase`) true))

(event `LeapEventInterface.LeapRightHandMoved`
  (params (Hand :type "LeapHand Object Reference"))
  (bind _right (`AnimBody.Right` (`self.AnimBody`)))
  (`AnimHand.SetFromLeapHand` _right Hand)
  (`AnimHand.ChangeBasis` _right (`self.RightPreBase`) (`self.RightPostBase`) true))

(event `LeapEventInterface.HandCountChanged`
  (params (Count :type Integer))
  (`self.DetermineHandChange` Count))

(event `Key|One`
  (params (Key :type "Key Structure"))
  (:`Pressed`
    (bind _returnvalue (`LeapController.IsTrackingPaused` (`self.LeapController`)))
    (`KismetSystemLibrary.PrintString` (`KismetStringLibrary.Conv_BoolToString` _returnvalue))))

(event `Key|Two`
  (params (Key :type "Key Structure"))
  (:`Pressed`
    (`LeapController.SetTrackingPause` (`self.LeapController`) true)))

(event `Key|Three`
  (params (Key :type "Key Structure"))
  (:`Pressed`
    (`LeapController.SetTrackingPause` (`self.LeapController`) false)))

(event `LeapEventInterface.LeapMotionOnDisconnect`
  (`KismetSystemLibrary.PrintString` "LeapMotionDisconnect" true true (struct :`R` 1.0 :`B` 0.261079 :`A` 1.0)))

(fn `DetermineHandChange`
  (params (Count :type Integer))
  (bind _skeletalmesh (`self.SkeletalMesh`))
  (bind _skeletalmesh_2 (`self.SkeletalMesh`))
  (bind _animbody (`self.AnimBody`))
  (bind _animbody_2 (`self.AnimBody`))
  (bind _left (`AnimBody.Left` _animbody_2))
  (bind _right (`AnimBody.Right` _animbody_2))
  (bind _left_2 (`AnimBody.Left` _animbody))
  (bind _right_2 (`AnimBody.Right` _animbody))
  (`/Engine/EditorBlueprintResources/StandardMacros.CompareInt` Count 2 ; Both Hands Visible
    (:`==`
      (`AnimHand.SetEnabled` _left true)
      (`AnimHand.SetEnabled` _right true)
      (`SkinnedMeshComponent.UnHideBoneByName` _skeletalmesh_2 "lf_forearm_roll_a")
      (`SkinnedMeshComponent.UnHideBoneByName` _skeletalmesh_2 "rt_forearm_roll_a"))
    (:`<`
      (`/Engine/EditorBlueprintResources/StandardMacros.CompareInt` Count ; none
        (:`>`
          (bind _returnvalue (`LeapController.Frame` (`self.LeapController`) 0)) ; One Hand Visible, which one is it?\n一只手看得见，是哪一只？
          (bind _returnvalue_2 (`LeapFrame.Hands` _returnvalue))
          (for _index (range (`LeapHandList.Count` _returnvalue_2))
            (bind _returnvalue_3 (`LeapHandList.GetIndex` _returnvalue_2 _index))
            (switch `ELeapHandType` (`LeapHand.HandType` _returnvalue_3)
              (:`HAND_LEFT`
                (`AnimHand.SetEnabled` _left_2 true)
                (`AnimHand.SetEnabled` _right_2 false)
                (`SkinnedMeshComponent.UnHideBoneByName` _skeletalmesh "lf_forearm_roll_a")
                (`SkinnedMeshComponent.HideBoneByName` _skeletalmesh "rt_forearm_roll_a" "PBO_None"))
              (:`HAND_RIGHT`
                (`AnimHand.SetEnabled` _right_2 true)
                (`AnimHand.SetEnabled` _left_2 false)
                (`SkinnedMeshComponent.UnHideBoneByName` _skeletalmesh "rt_forearm_roll_a")
                (`SkinnedMeshComponent.HideBoneByName` _skeletalmesh "lf_forearm_roll_a" "PBO_None")))
            (set `AnimBody.Alpha` 1.0 _animbody)))
        (:`==`
          (`AnimHand.SetEnabled` _left false)
          (`AnimHand.SetEnabled` _right false)
          (`SkinnedMeshComponent.HideBoneByName` _skeletalmesh_2 "rt_forearm_roll_a" "PBO_None")
          (`SkinnedMeshComponent.HideBoneByName` _skeletalmesh_2 "lf_forearm_roll_a" "PBO_None"))))))

(fn `GetAnimBody`
  (returns (AnimBody :type "AnimBody Object Reference"))
  (return (`self.AnimBody`)))

(fn `UserConstructionScript`)