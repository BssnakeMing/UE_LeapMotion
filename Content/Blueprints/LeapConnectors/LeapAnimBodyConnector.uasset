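; Connector that feeds Leap Motion hand tracking and HMD camera pose into an AnimBody, for driving a rigged character's hands and head.
; Hand-move events copy data on authority only, shifting by a mode-dependent offset and optionally changing basis for rigging.
; Hand count changes toggle each anim hand.
; Tick updates the head and detects HMD state changes, which re-optimise Leap tracking and recompute offsets from sprite markers, mesh and camera offsets.
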(event `self.ReceiveBeginPlay`
  (`self.HandleHMDModeChange`))

(event `self.HandCountChanged`
  (params (Count :type Integer))
  (`self.DetermineHandChange` Count))

(event `self.LeapHandMoved`
  (params (Hand :type "LeapHand Object Reference"))
  (bind _animbody (`self.AnimBody`))
  (if (`self.HasAuthority`)
    (switch `ELeapHandType` (`LeapHand.HandType` Hand)
      (:`HAND_LEFT`
        (`self.SetAnimHandFromLeapHand` (`AnimBody.Left` _animbody) Hand (`self.LeftPreBase`) (`self.LeftPostBase`)))
      (:`HAND_RIGHT`
        (`self.SetAnimHandFromLeapHand` (`AnimBody.Right` _animbody) Hand (`self.RightPreBase`) (`self.RightPostBase`))))))

(event `self.ReceiveTick`
  (params (DeltaSeconds :type "Float (single-precision)"))
  (`self.SetAnimHeadFromHMDCamera`) ; Update hmd data for animhead
)

(fn `DetermineHandChange`
  (params (Count :type Integer))
  (bind _animbody (`self.AnimBody`))
  (bind _animbody_2 (`self.AnimBody`))
  (bind _left (`AnimBody.Left` _animbody_2))
  (bind _right (`AnimBody.Right` _animbody_2))
  (bind _left_2 (`AnimBody.Left` _animbody))
  (bind _right_2 (`AnimBody.Right` _animbody))
  (`/Engine/EditorBlueprintResources/StandardMacros.CompareInt` Count 2 ; Both Hands Visible
    (:`==`
      (`AnimHand.SetEnabled` _left true)
      (`AnimHand.SetEnabled` _right true))
    (:`<`
      (`/Engine/EditorBlueprintResources/StandardMacros.CompareInt` Count ; none
        (:`>`
          (bind _returnvalue (`LeapController.Frame` (`self.LeapController`) 0)) ; One Hand Visible, which one is it?\n一只手看得见，是哪一只？
          (bind _returnvalue_2 (`LeapFrame.Hands` _returnvalue))
          (for _index (range (`LeapHandList.Count` _returnvalue_2))
            (bind _returnvalue_3 (`LeapHandList.GetIndex` _returnvalue_2 _index))
            (switch `ELeapHandType` (`LeapHand.HandType` _returnvalue_3)
              (:`HAND_LEFT`
                (`AnimHand.SetEnabled` _left_2 true)
                (`AnimHand.SetEnabled` _right_2 false))
              (:`HAND_RIGHT`
                (`AnimHand.SetEnabled` _right_2 true)
                (`AnimHand.SetEnabled` _left_2 false)))
            (set `AnimBody.Alpha` 1.0 _animbody)))
        (:`==`
          (`AnimHand.SetEnabled` _left false)
          (`AnimHand.SetEnabled` _right false))))))

(fn `DisplayDebugHandIfEnabled`
  (params (Hand :type "AnimHand Object Reference"))
  (if (`self.DebugPreview`)
    (`/SimpleLeapMontion/Blueprints/Utility/DebugHandUtility.DebugFullHand` (`self.DebugHand`) Hand 1.0 (`self.LeapBaseOffset`))
    (`KismetSystemLibrary.DrawDebugBox` (`SceneComponent.K2_GetComponentLocation` (`self.DefaultModeSprite`)) (5.0 5.0 5.0) (struct :`G` 0.34 :`B` 0.03373 :`A` 1.0))))

(fn `GetOwnerComponentClass`
  (params (Type :type "ActorComponent Class Reference"))
  (returns (Component :type "SceneComponent Object Reference"))
  (bind `_as场景组件` (cast `SceneComponent` (`|GetArrayItem` (`self.K2_GetComponentsByClass` (`ActorComponent.GetOwner` (`SceneComponent.GetAttachParent` (`self.K2_GetRootComponent`))) Type)))
    (:`then`
      (return `_as场景组件`))
    (:`CastFailed`
      (return null))))

(fn `HandleHMDModeChange`
  (bind _compensateforhmd (`self.CompensateForHMD`))
  (bind _leapfacingmodeishmd (`self.LeapFacingModeIsHMD`))
  (`AnimBone.SetEnabled` (`AnimBody.Head` (`self.AnimBody`)) _leapfacingmodeishmd) ; Ensure we enable our anim body head when the state changes\n确保我们在状态改变时启用我们的动物身体头部
  (`LeapController.OptimizeForHMD` (`self.LeapController`) _leapfacingmodeishmd _compensateforhmd _compensateforhmd) ; Adjust leap tracking to match mode\n调整跳跃跟踪以匹配模式
  (`self.SetStaticOffsets`))

(fn `SetAnimHandFromLeapHand`
  (params (AnimHand :type "AnimHand Object Reference") (LeapHand :type "LeapHand Object Reference") (PreBase :type "Rotator Structure") (PostBase :type "Rotator Structure"))
  (`AnimHand.SetFromLeapHand` AnimHand LeapHand) ; Leap Convenience AnimHand Set Method\n跳跃方便动漫手部设置方法
  (`self.DisplayDebugHandIfEnabled` AnimHand) ; Display Debug Hands for reference if enabled\n如果启用，显示调试手以供参考
  (`AnimHand.TranslateHand` AnimHand (`self.AnimBodyOffset`)) ; Adjust for hmd/default mode base position\n调整hmd/默认模式基准位置
  ;[1 1 1] Rigged Model Adjustment (rotate for Y = forward)
  ; 索具模型调整（Y旋转=向前）
  (if (`self.UseRiggingBasisAdjustment`)
    (`AnimHand.ChangeBasis` AnimHand PreBase PostBase true) ; post base of 0,0,90 is a rotation to Y Forward\n柱底为0,0,90是向Y正向旋转
  ))

(fn `SetAnimHeadFromHMDCamera`
  (bind _hmd_camera_component (`self.HMD Camera Component`))
  (bind _head (`AnimBody.Head` (`self.AnimBody`)))
  (`|ExecutionSequence`
    (:`then_0`
      (if (`HeadMountedDisplayFunctionLibrary.IsHeadMountedDisplayEnabled`)
        (if (!= _hmd_camera_component null)
          (set `AnimBone.Position` (+ (`SceneComponent.RelativeLocation` _hmd_camera_component) (`self.AnimBodyOffset`)) _head)
          (set `AnimBone.Orientation` (`SceneComponent.RelativeRotation` (`self.HMD Camera Component`)) _head)
          ;[1 1 1] Rigging Basis Adjustments?
          ; 索具基础调整？
          (if (`self.UseRiggingBasisAdjustment`)
            (`AnimBone.ChangeBasis` _head (struct :`Pitch` 90.0 :`Roll` 90.0) (struct :`Yaw` 90.0) true))
          (else
            (`AnimBone.SetEnabled` _head false)))))
    (:`then_1`
      (`self.HasHMDStateChanged` ; Handle hmd mode changes
        (:`Changed`
          (`self.HandleHMDModeChange`))))))

(fn `SetIPDToDefault`
  (`KismetSystemLibrary.ExecuteConsoleCommand` "stereo reset" null))

(fn `SetIPDToLeap`
  (`KismetSystemLibrary.ExecuteConsoleCommand` "stereo e=0.04" null))

(fn `SetOwnerLinks`
  (params (HMDCameraOffset :type "Vector Structure") (HMDCameraComponent :type "CameraComponent Object Reference") (UseDefaultIPD :type Boolean :default false) (MeshOffset :type "Vector Structure"))
  (`|ExecutionSequence`
    (:`then_0`
      (set `self.HMD Camera Offset` HMDCameraOffset)
      (set `self.HMD Camera Component` HMDCameraComponent)
      (if UseDefaultIPD
        (`self.SetIPDToDefault`)
        (else
          (`self.SetIPDToLeap`))))
    (:`then_1`
      (set `self.MeshOffset` MeshOffset))
    (:`then_2`
      (`self.HandleHMDModeChange`))))

(fn `SetStaticOffsets`
  (if (`self.LeapFacingModeIsHMD`)
    (set `self.LeapBaseOffset` (`SceneComponent.RelativeLocation` (`self.HMDModeSprite`)))
    (else
      (set `self.LeapBaseOffset` (`SceneComponent.RelativeLocation` (`self.DefaultModeSprite`)))))
  (set `self.AnimBodyOffset` (+ (`self.LeapBaseOffset`) (`self.MeshOffset`) (`self.HMD Camera Offset`))))

(fn `UserConstructionScript`)