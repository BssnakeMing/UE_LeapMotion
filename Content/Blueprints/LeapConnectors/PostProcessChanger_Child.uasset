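; PostProcessChanger_Child is a Leap Motion connector Blueprint that toggles camera-image passthrough.
; EnablePassthrough sets the controller's image support, image events and gamma correction, gates a gesture on the swipe option, and clears the link-initialized flag so pointers reinitialize.
; The construction script shows the debug billboard only when image debugging is on.
; ShowPassthrough is an empty stub, and the PostProcessChanger reference is unused.
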(fn `EnablePassthrough`
  (params (Enable :type Boolean) (`Enable Swipe Gesture` :type Boolean))
  (bind _leapcontroller (`self.LeapController`))
  (bind _output_get (set `self.PassthroughEnabled` Enable))
  (`LeapController.EnableImageSupport` _leapcontroller _output_get _output_get (`self.UseGammaCorrection`))
  (`LeapController.EnableGesture` _leapcontroller "GESTURE_TYPE_INVALID" (and _output_get `Enable Swipe Gesture`))
  (set `self.PassthroughLinkInitialized` false) ; Pointers should reinitialize
)

(fn `ShowPassthrough`
  (params (Show :type Boolean))
  (if Show
    _))

(fn `UserConstructionScript`
  (bind _debugimages (`self.DebugImages`))
  (bind _debugbillboard (`self.DebugBillboard`))
  ;[1 1 1] Hide the debug billboard if we're not debugging
  (`SceneComponent.SetVisibility` _debugbillboard _debugimages false)
  (`SceneComponent.SetHiddenInGame` _debugbillboard (not _debugimages) false))